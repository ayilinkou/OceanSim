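; BP_Boat is a boat actor that bobs up and down and sways in place.
; On BeginPlay it caches its starting transform and plays UpDownTimeline, restarting it whenever it finishes for an endless loop.
; Each update offsets the starting location by the scaled height track and sets roll and pitch from scaled sway tracks.
; Rotation is absolute with yaw forced to zero, so the placed rotation is not preserved.
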(event `self.ReceiveBeginPlay`
  (set `self.InitialTransform` (`self.GetTransform`))
  (`|ExecutionSequence`
    (:`then_0`
      (bind (_direction _height _swaypitch _swayroll) (`Timeline|UpDownTimeline` :!label _label)
        (:`Update`
          (`self.K2_SetActorLocation` (+ (* (`self.HeightMaxOffset`) _height) (.location (`self.InitialTransform`))))
          (`self.K2_SetActorRotation` (`KismetMathLibrary.MakeRotator` (* (* _swayroll -1.0) (`self.SwayAngleRoll`)) (* _swaypitch (`self.SwayAnglePitch`)))))
        (:`Finished`
          (goto _label :!via `PlayFromStart`))))))

(fn `UserConstructionScript`)